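; BP_Sheep is the player character of a sheep microgame, running automatically along negative world Y and jumping over a hurdle on input.
; Each tick it feeds Speed into movement input and checks whether the Hurdle lies behind it on Y and over a set distance away, which clears the microgame.
; A capsule hit against BP_Hurdle fails it.
; Both outcomes only zero Speed and print a message.
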(event OnComponentHit(CapsuleComponent)
  (params (HitComponent :type Primitive%20Component%20Object%20Reference) (OtherActor :type Actor%20Object%20Reference) (OtherComp :type Primitive%20Component%20Object%20Reference) (NormalImpulse :type Vector :default "0, 0, 0") (Hit :type Hit%20Result%20Structure%20%28by%20ref%29))
  (Utilities|Casting|CastToBP_Hurdle OtherActor)
  (CallFunction|MicrogameFailed))

(event EventBeginPlay)

(event Collision|EventActorBeginOverlap
  (params (OtherActor :type Actor%20Object%20Reference)))

(event EventTick
  (params (DeltaSeconds :type Float%20%28single-precision%29))
  (CallFunction|SheepRunTick)
  (CallFunction|CheckVictory))

(event Input|ActionEvents|InputActionSheep_Jump
  (params (Key :type Key%20Structure :default "None"))
  (:Pressed
    (Character|Jump))
  (:Released
    (Character|StopJumping)))

(fn ConstructionScript)

(fn SheepRunTick
  (Class|PawnMovementComponent|AddInputVector (Variables|Character|GetCharacterMovement) (Math|Vector|MakeVector 0.0 (* (Variables|Default|GetSpeed) -1.0) 0.0) false))

(fn MicrogameClear
  (Variables|Default|SetSpeed 0.0)
  (Development|PrintText "clear"))

(fn MicrogameFailed
  (Variables|Default|SetSpeed 0.0)
  (Development|PrintText "Failed"))

(fn CheckVictory
  (bind _hurdle (Variables|Default|GetHurdle))
  (Utilities|IsValid _hurdle
    (:Is%20Valid
      (if (and (> (Transformation|GetDistanceTo _hurdle) 5e+02) (> (.y (Transformation|GetActorLocation _hurdle)) (.y (Transformation|GetActorLocation))))
        (CallFunction|MicrogameClear)))))